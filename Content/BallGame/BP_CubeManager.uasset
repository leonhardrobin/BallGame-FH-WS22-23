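; Manager actor for a cube-shooting game that spawns one moving cube at a time, starting at BeginPlay.
; Each cube gets a randomized navmesh-based position with random height, axis-aligned velocity, size and travel distance, using GameInstance ranges for speed and size.
; OnCubeDestroyed updates the shot count and notifies the GameMode, then spawns another cube or, at the target count, writes cached statistics and opens the Entry level.
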(event `self.ReceiveBeginPlay`
  (`self.SpawnMovingCube`)
  (`KismetSystemLibrary.PrintString` "Hello"))

(event `OnCubeDestroyed`
  (`/Engine/EditorBlueprintResources/StandardMacros.IncrementInt` (`self.NumCubesShot`)
    (:`  `
      (bind _asbp_first_person_game_mode (cast `/Game/BallGame/BP_FirstPersonGameMode` (`GameplayStatics.GetGameMode`)))
      (`/Game/BallGame/BP_FirstPersonGameMode.OnCubeShot` _asbp_first_person_game_mode (`self.NumCubesShot`))
      (bind _asbp_game_instance (cast `/Game/BallGame/UI/BP_GameInstance` (`GameplayStatics.GetGameInstance`)))
      (if (>= (`self.NumCubesShot`) (`/Game/BallGame/UI/BP_GameInstance.NumCubesToShoot` _asbp_game_instance))
        (`StatisticsSubsystem.WriteCachedCubeInfo` (subsystem `StatisticsSubsystem`))
        (`GameplayStatics.OpenLevelBySoftObjectPtr` "/Game/Maps/Entry.Entry")
        (else
          (`self.SpawnMovingCube`))))))

(fn `GetRandomSize`
  (returns (Size :type "Vector Structure"))
  (bind _asbp_game_instance (cast `/Game/BallGame/UI/BP_GameInstance` (`GameplayStatics.GetGameInstance`)))
  (bind _returnvalue (`KismetMathLibrary.RandomFloatInRange` (`/Game/BallGame/UI/BP_GameInstance.Cube Size Min` _asbp_game_instance) (`/Game/BallGame/UI/BP_GameInstance.Cube Size Max` _asbp_game_instance)))
  (return (`KismetMathLibrary.MakeVector` _returnvalue _returnvalue _returnvalue)))

(fn `GetRandomSpawnTransform`
  (returns (SpawnTransform :type "Transform Structure"))
  (bind _randomlocation (`NavigationSystemV1.K2_GetRandomReachablePointInRadius` (`self.K2_GetActorLocation`) 3000.0 null null))
  (return (`KismetMathLibrary.MakeTransform` (`KismetMathLibrary.MakeVector` (.x _randomlocation) (.y _randomlocation) (`KismetMathLibrary.RandomFloatInRange` 200.0 500.0)))))

(fn `GetRandomVelocity`
  (returns (Velocity :type "Vector Structure"))
  (bind _asbp_game_instance (cast `/Game/BallGame/UI/BP_GameInstance` (`GameplayStatics.GetGameInstance`)))
  (return (* (select `int` (`KismetMathLibrary.RandomIntegerInRange` 0 2) :`0` (`KismetMathLibrary.MakeVector` 1.0) :`1` (`KismetMathLibrary.MakeVector` 0.0 1.0) :`2` (`KismetMathLibrary.MakeVector` 0.0 0.0 1.0)) (`KismetMathLibrary.RandomFloatInRange` (`/Game/BallGame/UI/BP_GameInstance.Cube Speed Min` _asbp_game_instance) (`/Game/BallGame/UI/BP_GameInstance.Cube Speed Max` _asbp_game_instance)))))

(fn `SpawnMovingCube`
  (`|SpawnActorFromClass` "/Game/BallGame/BP_MovingCube.BP_MovingCube_C" (`self.GetRandomSpawnTransform`) "Undefined" "OverrideRootScale" null (* (`self.GetRandomVelocity`) (`self.CubeVelocityMultiplier`)) (`self.GetRandomSize`) (`KismetMathLibrary.RandomFloatInRange` 70.0 500.0) null))

(fn `UserConstructionScript`)