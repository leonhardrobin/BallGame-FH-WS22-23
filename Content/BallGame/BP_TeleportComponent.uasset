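; Scene component that lets its owning actor teleport by aiming along the component's forward vector, with a spawned BP_TeleportTarget as the marker.
; While teleporting, each tick it line-traces forward, projects the hit onto the navmesh and moves the marker there.
; StartTeleport shows the marker.
; EndTeleport hides it and, if a valid point was found, moves the owner there, raised by its capsule half height.
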(event `self.ReceiveBeginPlay`
  (bind _returnvalue (`|SpawnActorFromClass` "/Game/BallGame/BP_TeleportTarget.BP_TeleportTarget_C" (`KismetMathLibrary.MakeTransform` (0.0 0.0 0.0)) "Undefined" "OverrideRootScale" null null))
  (set `self.Target` _returnvalue)
  (bind _output_get (set `self.ActorToTeleport` (`self.GetOwner`)))
  (bind _returnvalue_2 (`Actor.GetComponentByClass` _output_get "/Script/Engine.CapsuleComponent"))
  (`/Engine/EditorBlueprintResources/StandardMacros.IsValid` _returnvalue_2
    (:`Is Valid`
      (set `self.Capsule Half Height` (`CapsuleComponent.CapsuleHalfHeight` _returnvalue_2)))))

(event `self.ReceiveTick`
  (params (DeltaSeconds :type "Float (single-precision)"))
  (if (`self.bIsTeleporting`)
    (`self.DetectHitPoint`)))

(fn `DetectHitPoint`
  (bind _returnvalue (`self.K2_GetComponentLocation`))
  (bind (_outhit _returnvalue_2) (`KismetSystemLibrary.LineTraceSingle` _returnvalue (+ _returnvalue (* (`self.distance`) (`self.GetForwardVector`))) "TraceTypeQuery1"))
  (bind (_projectedlocation _returnvalue_3) (`NavigationSystemV1.K2_ProjectPointToNavigation` (`.Location` (`GameplayStatics.BreakHitResult` _outhit))))
  (set `self.bHitDetected` (and _returnvalue_3 _returnvalue_2))
  (bind _output_get (set `self.Hit Location` _projectedlocation))
  (`Actor.K2_SetActorLocation` (`self.Target`) _output_get false false))

(fn `EndTeleport`
  (bind (_hit_location_x _hit_location_y _hit_location_z) (`KismetMathLibrary.BreakVector` (`self.Hit Location`)))
  (`self.SetVisibility` (`/Game/BallGame/BP_TeleportTarget.Sphere` (`self.Target`)) false false)
  (set `self.bIsTeleporting` false)
  (if (`self.bHitDetected`)
    (`Actor.K2_SetActorLocation` (`self.ActorToTeleport`) (`KismetMathLibrary.MakeVector` _hit_location_x _hit_location_y (+ _hit_location_z (`self.Capsule Half Height`))) false false)))

(fn `StartTeleport`
  (set `self.bIsTeleporting` true)
  (`self.SetVisibility` (`/Game/BallGame/BP_TeleportTarget.Sphere` (`self.Target`)) true false))